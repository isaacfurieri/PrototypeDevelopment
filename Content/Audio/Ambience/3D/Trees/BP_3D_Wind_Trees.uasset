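; BP_3D_Wind_Trees is a 3D ambience emitter for wind in trees, triggered by player proximity.
; The construction script applies a MetaSound, attenuation settings and sphere radius from variables to the audio component and collision sphere.
; When BP_ThirdPersonCharacter begins overlapping the sphere, it prints a debug message and plays the sound from the start.
; The graph has no end-overlap handler to stop playback.
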(event `self.TreesSphereCollision.OnComponentBeginOverlap`
  (params (OverlappedComponent :type "PrimitiveComponent Object Reference") (OtherActor :type "Actor Object Reference") (OtherComp :type "PrimitiveComponent Object Reference") (OtherBodyIndex :type Integer) (bFromSweep :type Boolean) (SweepResult :type "HitResult Structure (by ref)"))
  (cast `/Game/ThirdPerson/Blueprints/BP_ThirdPersonCharacter` OtherActor)
  (`KismetSystemLibrary.PrintString` "Detecting ambience sphere")
  (`AudioComponent.Play` (`self.3DWindTreesComponent`) 0.0))

(fn `UserConstructionScript`
  (`AudioComponent.SetSound` (`self.3DWindTreesComponent`) (`self.MetaSoundVar`))
  (set `AudioComponent.AttenuationSettings` (`self.SoundAttenVar`) (`self.3DWindTreesComponent`))
  (`SphereComponent.SetSphereRadius` (`self.TreesSphereCollision`) (`self.SphereRadiusVar`) true))