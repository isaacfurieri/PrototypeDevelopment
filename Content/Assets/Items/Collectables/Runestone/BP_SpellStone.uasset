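; Collectable runestone (spell stone) pickup that spins every tick and is collected on any overlap with its box.
; Pickup plays a sound at the player, increments the GameProgress game instance's SpellStones count, and records the stone's ID there.
; HideCollected, matched by ID, hides the mesh and indicator sprite and disables collision instead of destroying the actor.
; Debug prints report the hidden stone and announce when all 102 are collected.
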(event `self.ReceiveTick`
  (params (DeltaSeconds :type "Float (single-precision)"))
  (`SceneComponent.K2_AddLocalRotation` (`self.RuneStone`) (struct :`Yaw` 5.0) false false))

(event `self.Box.OnComponentBeginOverlap`
  (params (OverlappedComponent :type "PrimitiveComponent Object Reference") (OtherActor :type "Actor Object Reference") (OtherComp :type "PrimitiveComponent Object Reference") (OtherBodyIndex :type Integer) (bFromSweep :type Boolean) (SweepResult :type "HitResult Structure (by ref)"))
  (bind _id (`self.ID`))
  (`GameplayStatics.PlaySoundAtLocation` "/Game/Audio/Collectibles/MS_Pickup_Runestone.MS_Pickup_Runestone" (`self.K2_GetActorLocation` (`GameplayStatics.GetPlayerPawn` 0)) (struct) 1.0 1.0 0.0 null null null null)
  (bind _asgame_progress (cast `/Game/GameProgress` (`GameplayStatics.GetGameInstance`)))
  (set `/Game/GameProgress.SpellStones` (+ (`/Game/GameProgress.SpellStones` _asgame_progress) 1) _asgame_progress)
  (bind _asgame_progress_2 (cast `/Game/GameProgress` (`GameplayStatics.GetGameInstance`)))
  (`/Game/GameProgress.RunestoneCollected` _asgame_progress_2 _id)
  (`self.HideCollected` self _id)
  (bind _asgame_progress_3 (cast `/Game/GameProgress` (`GameplayStatics.GetGameInstance`)))
  (if (== (`/Game/GameProgress.SpellStones` _asgame_progress_3) 102)
    (`KismetSystemLibrary.PrintString` "ALL SPELLSTONES COLLECTED!!!" true true (struct :`R` 1.0 :`B` 0.694118 :`A` 1.0) 5.0)))

(event `HideCollected`
  (params (ID_SpellStone :type Integer))
  ;[1 1 1] Hide Item when collected and Set no collision
  (if (== ID_SpellStone (`self.ID`))
    (`SceneComponent.SetVisibility` (`self.RuneStone`) false false)
    (`PrimitiveComponent.SetCollisionEnabled` (`self.Box`) "NoCollision")
    (`PrimitiveComponent.SetCollisionEnabled` (`self.RuneStone`) "NoCollision")
    (`SceneComponent.SetVisibility` (`self.ItemIndicatorSprite`) false false)
    (`KismetSystemLibrary.PrintString` (`KismetStringLibrary.Concat_StrStr` (`KismetStringLibrary.Conv_IntToString` (`self.ID`)) " Set to Invisible " (`KismetSystemLibrary.GetObjectName` self)) true true (struct :`G` 0.102339 :`B` 1.0 :`A` 1.0) 10.0)))

(fn `UserConstructionScript`)