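; Golden Feather collectable that spins in the world and upgrades the player's glide when picked up.
; On box overlap it plays a pickup sound, hides itself and increments the feather count in the GameProgress game instance.
; That count sets the strength passed to the third-person character's GlidePowerUp.
; HideCollected matches a feather ID before turning off visibility, collision and the indicator sprite.
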(event `self.ReceiveTick`
  (params (DeltaSeconds :type "Float (single-precision)"))
  ;[1 1 1] Golden Feather Mesh Rotation
  (`SceneComponent.K2_AddLocalRotation` (`self.FeatherHandle`) (struct :`Yaw` 5.0) false false))

(event `self.Box.OnComponentBeginOverlap`
  (params (OverlappedComponent :type "PrimitiveComponent Object Reference") (OtherActor :type "Actor Object Reference") (OtherComp :type "PrimitiveComponent Object Reference") (OtherBodyIndex :type Integer) (bFromSweep :type Boolean) (SweepResult :type "HitResult Structure (by ref)"))
  ;[1 1 1] Collection mechanics
  (`GameplayStatics.PlaySoundAtLocation` "/Game/Audio/Collectibles/MS_Pickup_GoldenFeather.MS_Pickup_GoldenFeather" (`self.K2_GetActorLocation` (`GameplayStatics.GetPlayerPawn` 0)) (struct) 1.0 1.0 0.0 null null null null)
  (bind _asgame_progress (cast `/Game/GameProgress` (`GameplayStatics.GetGameInstance`)))
  (`self.HideCollected` self (`self.ID`))
  (bind _output_get (set `/Game/GameProgress.GoldenFeathers` (+ (`/Game/GameProgress.GoldenFeathers` _asgame_progress) 1) _asgame_progress))
  (bind _asbp_third_person_character (cast `/Game/ThirdPerson/Blueprints/BP_ThirdPersonCharacter` (`GameplayStatics.GetPlayerCharacter` 0)))
  (if (>= _output_get 0)
    (bind _returnvalue (* _output_get 0.3))
    (`/Game/ThirdPerson/Blueprints/BP_ThirdPersonCharacter.GlidePowerUp` _asbp_third_person_character (+ 1.0 _returnvalue))
    (else
      (`/Game/ThirdPerson/Blueprints/BP_ThirdPersonCharacter.GlidePowerUp` _asbp_third_person_character _returnvalue))))

(event `HideCollected`
  (params (ID_GF :type Integer))
  ;[1 1 1] Hide Item when collected and Set no collision
  (if (== ID_GF (`self.ID`))
    (`SceneComponent.SetVisibility` (`self.GoldenFeather`) false false)
    (`SceneComponent.SetVisibility` (`self.FeatherHandle`) false false)
    (`PrimitiveComponent.SetCollisionEnabled` (`self.Box`) "NoCollision")
    (`PrimitiveComponent.SetCollisionEnabled` (`self.GoldenFeather`) "NoCollision")
    (`PrimitiveComponent.SetCollisionEnabled` (`self.FeatherHandle`) "NoCollision")
    (`SceneComponent.SetVisibility` (`self.ItemIndicatorSprite`) false false)))

(fn `UserConstructionScript`)